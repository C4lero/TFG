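; Dialogue component that runs data-table-driven branching conversations in a crisis game with time and tension stakes.
; Interact opens or advances WB_Dialogue, with each row pointing to the next and open-ended rows spawning WB_Options buttons that report through OptionSelected.
; Advancing or selecting adds time, tension and notepad text to GI_CrisisGameInstance, then CheckCrisisState shows WB_GameOver at either limit.
; Ending or leaving dialogue restores game input and clears the player's Talking flag.
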(event `CheckCrisisState`
  (`KismetSystemLibrary.PrintString` "activo vigilante")
  (bind _asgi_crisis_game_instance (cast `/Game/Blueprints/GI_CrisisGameInstance` (`GameplayStatics.GetGameInstance`)))
  (if (>= (`/Game/Blueprints/GI_CrisisGameInstance.TensionPoints` _asgi_crisis_game_instance) 100)
    (`KismetSystemLibrary.PrintString` "la tension es 100")
    (bind _returnvalue (`|CreateWidget` "/Game/Blueprints/WB_GameOver.WB_GameOver_C" null "has perdido por perder el control"))
    (`UserWidget.AddToViewport` _returnvalue 0)
    (elif (>= (`/Game/Blueprints/GI_CrisisGameInstance.CurrentTime` _asgi_crisis_game_instance) (`/Game/Blueprints/GI_CrisisGameInstance.LimitTime` _asgi_crisis_game_instance))
      (bind _returnvalue_2 (`|CreateWidget` "/Game/Blueprints/WB_GameOver.WB_GameOver_C" null "has perdidio por tiempo"))
      (`UserWidget.AddToViewport` _returnvalue_2 0))))

(event `OptionSelected`
  (params (DataTable :type "DataTable Object Reference") (RowName :type Name))
  (bind _dialoguewidget (`self.DialogueWidget`))
  (bind _returnvalue (`|GetDataTableRow` DataTable RowName)
    (:`then`
      (bind _asgi_crisis_game_instance (cast `/Game/Blueprints/GI_CrisisGameInstance` (`GameplayStatics.GetGameInstance`)))
      (bind (_dialogue _row _datatable _enddialogue_ _openendeddialogue_ _openendeddialogueoptions _timecost _tensionmodifier _relevanttext) (break `/Game/Dialogue/Dialogue_Structure` _returnvalue))
      (bind _output_get (set `/Game/Blueprints/GI_CrisisGameInstance.CurrentTime` (`KismetMathLibrary.FTrunc` (+ (`/Game/Blueprints/GI_CrisisGameInstance.CurrentTime` _asgi_crisis_game_instance) _timecost)) _asgi_crisis_game_instance))
      ; Variable update debug when options
      (`KismetSystemLibrary.PrintString` "CURRENT TIME")
      (`KismetSystemLibrary.PrintString` (`KismetStringLibrary.Conv_DoubleToString` (`KismetMathLibrary.Conv_IntToDouble` _output_get)))
      (bind _output_get_2 (set `/Game/Blueprints/GI_CrisisGameInstance.TensionPoints` (+ (`/Game/Blueprints/GI_CrisisGameInstance.TensionPoints` _asgi_crisis_game_instance) _tensionmodifier) _asgi_crisis_game_instance))
      (`KismetSystemLibrary.PrintString` "CURRENT TIME")
      (`KismetSystemLibrary.PrintString` (`KismetStringLibrary.Conv_IntToString` _output_get_2))
      (`self.CheckCrisisState`)
      (if (`KismetStringLibrary.NotEqual_StrStr` (`KismetTextLibrary.Conv_TextToString` _relevanttext))
        (`KismetSystemLibrary.PrintString` "TEXT AADDED")
        (`KismetSystemLibrary.PrintString` (`KismetTextLibrary.Conv_TextToString` _relevanttext))
        (`KismetArrayLibrary.Array_Add` (`/Game/Blueprints/GI_CrisisGameInstance.Notepad` _asgi_crisis_game_instance) _relevanttext))
      (`PanelWidget.ClearChildren` (`/Game/Dialogue/WB_Dialogue.OptionScrollBox` _dialoguewidget))
      (`/Game/Dialogue/WB_Dialogue.Update Dialog` _dialoguewidget _dialogue)
      (set `self.Row Name` _row)
      (set `self.Data Table` _datatable)
      (set `self.EndDialogue` _enddialogue_)
      ; if we want to respond to a selection with another selection
      (if _openendeddialogue_
        (for _array_element _openendeddialogueoptions
          (bind (_optionname _row_2 _datatable_2) (break `/Game/Dialogue/OptionsDialogue_Structure` _array_element))
          (bind _returnvalue_2 (`|CreateWidget` "/Game/Dialogue/WB_Options.WB_Options_C" null (`KismetTextLibrary.Conv_NameToText` _optionname) self _row_2 _datatable_2))
          (`PanelWidget.AddChild` (`/Game/Dialogue/WB_Dialogue.OptionScrollBox` (`self.DialogueWidget`)) _returnvalue_2))))))

(event `/Game/Dialogue/BP_Interact.LeaveDialogue`
  (bind _returnvalue (`GameplayStatics.GetPlayerController` 0))
  (`/Engine/EditorBlueprintResources/StandardMacros.IsValid` (`self.DialogueWidget`)
    (:`Is Valid`
      ; Hiding dialogue widget
      (`Widget.RemoveFromParent` (`self.DialogueWidget`) :!label _label)
      (set `self.EndDialogue` false)
      (set `self.DialogueWidget` null)
      (`WidgetBlueprintLibrary.SetInputMode_GameOnly` _returnvalue)
      (set `PlayerController.bShowMouseCursor` false _returnvalue)
      (bind _asbp_kid_red (cast `/Game/Blueprints/KidRed/BP_KidRed` (`GameplayStatics.GetPlayerCharacter` 0)))
      (set `/Game/Blueprints/KidRed/BP_KidRed.Talking` false _asbp_kid_red))))

(event `/Game/Dialogue/BP_Interact.Interact`
  (params (PlayerReference :type "/Game/Blueprints/KidRed/BP_KidRed Object Reference"))
  (bind _returnvalue (`GameplayStatics.GetPlayerController` 0))
  (bind _notepadref (`/Game/Blueprints/KidRed/BP_KidRed.NotepadRef` PlayerReference))
  (`/Engine/EditorBlueprintResources/StandardMacros.IsValid` _notepadref
    (:`Is Valid`
      (`Widget.RemoveFromParent` _notepadref))
    (:`Is Not Valid`
      _))
  (set `/Game/Blueprints/KidRed/BP_KidRed.Talking` true PlayerReference)
  (if (`self.EndDialogue`)
    (goto _label)
    (else
      (`/Engine/EditorBlueprintResources/StandardMacros.IsValid` (`self.DialogueWidget`)
        (:`Is Valid`
          (bind _returnvalue_2 (`|GetDataTableRow` (`self.Data Table`) (`self.Row Name`))
            (:`then`
              (bind _asgi_crisis_game_instance (cast `/Game/Blueprints/GI_CrisisGameInstance` (`GameplayStatics.GetGameInstance`)))
              (bind (_dialogue _row _datatable _enddialogue_ _openendeddialogue_ _openendeddialogueoptions _timecost _tensionmodifier _relevanttext) (break `/Game/Dialogue/Dialogue_Structure` _returnvalue_2))
              (bind _output_get (set `/Game/Blueprints/GI_CrisisGameInstance.CurrentTime` (+ (`/Game/Blueprints/GI_CrisisGameInstance.CurrentTime` _asgi_crisis_game_instance) _timecost) _asgi_crisis_game_instance))
              ; Variable update debug
              (`KismetSystemLibrary.PrintString` "CURRENT TIME")
              (`KismetSystemLibrary.PrintString` (`KismetStringLibrary.Conv_DoubleToString` (`KismetMathLibrary.Conv_IntToDouble` _output_get)))
              (bind _output_get_2 (set `/Game/Blueprints/GI_CrisisGameInstance.TensionPoints` (+ (`/Game/Blueprints/GI_CrisisGameInstance.TensionPoints` _asgi_crisis_game_instance) _tensionmodifier) _asgi_crisis_game_instance))
              (`KismetSystemLibrary.PrintString` "CURRENT TIME")
              (`KismetSystemLibrary.PrintString` (`KismetStringLibrary.Conv_IntToString` _output_get_2))
              (`self.CheckCrisisState`)
              (if (`KismetStringLibrary.NotEqual_StrStr` (`KismetTextLibrary.Conv_TextToString` _relevanttext))
                (`KismetSystemLibrary.PrintString` "TEXT AADDED")
                (`KismetSystemLibrary.PrintString` (`KismetTextLibrary.Conv_TextToString` _relevanttext))
                (`KismetArrayLibrary.Array_Add` (`/Game/Blueprints/GI_CrisisGameInstance.Notepad` _asgi_crisis_game_instance) _relevanttext))
              (`/Game/Dialogue/WB_Dialogue.Update Dialog` (`self.DialogueWidget`) _dialogue)
              (set `self.Row Name` _row)
              (set `self.Data Table` _datatable)
              (set `self.EndDialogue` _enddialogue_))))
        (:`Is Not Valid`
          (bind _returnvalue_3 (`|GetDataTableRow` (`self.Data Table`) (`self.Row Name`))
            (:`then`
              (bind (_dialogue_2 _row_2 _datatable_2 _enddialogue__2 _openendeddialogue__2 _openendeddialogueoptions_2) (break `/Game/Dialogue/Dialogue_Structure` _returnvalue_3))
              (bind _returnvalue_4 (`|CreateWidget` "/Game/Dialogue/WB_Dialogue.WB_Dialogue_C" null (`KismetTextLibrary.Conv_NameToText` (`self.Name`)) _dialogue_2))
              (bind _output_get_3 (set `self.DialogueWidget` _returnvalue_4))
              (`UserWidget.AddToViewport` _output_get_3 0)
              (set `self.Row Name` _row_2)
              (set `self.Data Table` _datatable_2)
              (set `self.EndDialogue` _enddialogue__2)
              (`WidgetBlueprintLibrary.SetInputMode_GameAndUIEx` _returnvalue null)
              (set `PlayerController.bShowMouseCursor` true _returnvalue)
              (if _openendeddialogue__2
                (for _array_element _openendeddialogueoptions_2
                  (bind (_optionname _row_3 _datatable_3) (break `/Game/Dialogue/OptionsDialogue_Structure` _array_element))
                  (bind _returnvalue_5 (`|CreateWidget` "/Game/Dialogue/WB_Options.WB_Options_C" null (`KismetTextLibrary.Conv_NameToText` _optionname) self _row_3 _datatable_3))
                  (`PanelWidget.AddChild` (`/Game/Dialogue/WB_Dialogue.OptionScrollBox` (`self.DialogueWidget`)) _returnvalue_5))))))))))